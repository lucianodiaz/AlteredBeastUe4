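; Enemy Character for a side-scrolling Altered Beast game, apparently a shared base, with health, delayed activation and knockback.
; Unless stopped, Tick locks Y to a middle lane, nudges X minutely as fake movement and flags upward motion as airborne.
; StartEvent flags spawning, unhides it and restores collision, plus gravity where allowed.
; Only LoboProyectil damage reduces health; knockback jumps and shifts it along +X, while the Player1 hit check does nothing.
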(event `movimientoFalso`
  (`self.K2_SetActorLocation` (`KismetMathLibrary.MakeVector` (+ (.x (`self.K2_GetActorLocation`)) 0.001) (.y (`self.K2_GetActorLocation`)) (.z (`self.K2_GetActorLocation`)))))

(event `self.ReceiveTick`
  (params (DeltaSeconds :type "Float (single-precision)"))
  (bind (_returnvalue_x _returnvalue_y _returnvalue_z) (`KismetMathLibrary.BreakVector` (`self.GetVelocity`)))
  (if (not (`self.Stop`))
    (`self.StayInTheMiddle`)
    (`self.movimientoFalso`)
    (set `self.inTheAir` (> _returnvalue_z 0.0))))

(event `self.ReceiveAnyDamage`
  (params (Damage :type "Float (single-precision)") (DamageType :type "DamageType Object Reference") (InstigatedBy :type "Controller Object Reference") (DamageCauser :type "Actor Object Reference"))
  (cast `/Game/AlteredBeast/Blueprints/Players/proyectile/LoboProyectil` DamageCauser)
  (set `self.vida` (- (`self.vida`) Damage)))

(event `Mostrar`
  (`self.SetActorHiddenInGame` false)
  (if (not (`self.NoGravity?`))
    (set `CharacterMovementComponent.GravityScale` 1.0 (`self.CharacterMovement`)))
  (`PrimitiveComponent.SetCollisionEnabled` (`self.CapsuleComponent`) "QueryAndPhysics"))

(event `ActivarSpawn`
  (if (`self.Start`)
    (set `self.bSpawn` true)))

(event `StartEvent`
  (set `self.Start` true)
  (`self.ActivarSpawn`)
  (`self.Mostrar`))

(event `self.CapsuleComponent.OnComponentHit`
  (params (HitComponent :type "PrimitiveComponent Object Reference") (OtherActor :type "Actor Object Reference") (OtherComp :type "PrimitiveComponent Object Reference") (NormalImpulse :type "Vector Structure") (Hit :type "HitResult Structure (by ref)"))
  (cast `/Game/AlteredBeast/Blueprints/Player1` OtherActor))

(event `knockbackSalto`
  (if (not (`self.InTheAir`))
    (`self.Jump`)))

(event `volar`
  (`self.knockbackSalto`)
  (set `self.InTheAir` true)
  (`self.K2_SetActorLocation` (`KismetMathLibrary.MakeVector` (+ (.x (`self.K2_GetActorLocation`)) 1.2) (.y (`self.K2_GetActorLocation`)) (.z (`self.K2_GetActorLocation`))) true))

(fn `StayInTheMiddle`
  (`self.K2_SetActorLocation` (`KismetMathLibrary.MakeVector` (.x (`self.K2_GetActorLocation`)) (`self.middle`) (.z (`self.K2_GetActorLocation`)))))

(fn `UserConstructionScript`)