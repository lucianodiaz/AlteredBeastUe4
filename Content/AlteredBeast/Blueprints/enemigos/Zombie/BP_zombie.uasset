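; Side-scrolling Altered Beast zombie enemy that rises from the ground once started, walks toward a Player1, then charges and explodes when close.
; Tick runs the behavior through boolean flags for spawning, movement, knockback, hits, charging and explosion damage.
; Player or LoboProyectil hits drain health, switching it to headless animations, then to death with spawned body pieces.
; An enum selects the Paper2D flipbook, whose duration also times state resets.
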(event `self.ReceiveBeginPlay`
  (`parent.ReceiveBeginPlay`)
  (bind _outactors (`GameplayStatics.GetAllActorsOfClass` "/Game/AlteredBeast/Blueprints/Player1.Player1_C"))
  (for _array_element _outactors
    (if (`/Game/AlteredBeast/Blueprints/Player1.Aparecer` _array_element)
      (set `self.Player` _array_element)
      (`PrimitiveComponent.SetCollisionEnabled` (`self.explosion`) "NoCollision")
      (`PrimitiveComponent.SetCollisionEnabled` (`self.CapsuleComponent`) "NoCollision"))))

(event `StopFight`
  ;[1 1 1] Desactiva los golpes
  (bind _outflipbook (`self.EnumManager`))
  (if (`self.explode`)
    (bind _returnvalue (`PaperFlipbook.GetTotalDuration` _outflipbook))
    (`KismetSystemLibrary.Delay` _returnvalue)
    (`|ExecutionSequence`
      (:`then_0`
        (`GameplayStatics.PlaySoundAtLocation` (`self.sfx_explosion`)))
      (:`then_1`
        (set `self.explode` false)))
    (elif (`self.recharg`)
      (`KismetSystemLibrary.Delay` _returnvalue)
      (set `self.recharg` false)
      (set `self.explode` true)
      (elif (`self.isHit?`)
        (`KismetSystemLibrary.Delay` _returnvalue)
        (set `self.isHit?` false)))))

(event `self.ReceiveTick`
  (params (DeltaSeconds :type "Float (single-precision)"))
  ;[1 1 1] EVERY TICK
  (`parent.ReceiveTick` DeltaSeconds)
  (if (not (`self.Stop`))
    (`self.ChosePlayer`)
    (`self.SpawnEnemy`)
    (`self.ActivarZombi`)
    (`self.IsDead`)
    (`self.ManejoAnimacion`)
    (`self.knockBack`)
    (`self.StopFight`)
    (`self.noHead`)
    (`self.Explotar`)
    (`self.moveTo`)
    (`self.distance`)
    (`self.ActiveDesactive`)))

(event `IsDead`
  ;[1 1 1] death
  (if (<= (`self.vida`) 0.0)
    (set `self.isDead?` true)
    (`GameplayStatics.PlaySoundAtLocation` (`self.sfx_muerte`))))

(event `knockBack`
  (bind (_returnvalue_x _returnvalue_y _returnvalue_z) (`KismetMathLibrary.BreakVector` (`self.K2_GetActorLocation`)))
  (bind (_returnvalue_x_2 _returnvalue_y_2 _returnvalue_z_2) (`KismetMathLibrary.BreakVector` (`self.GetVelocity`)))
  (bind _returnvalue_x_3 (`KismetMathLibrary.BreakVector` (`self.K2_GetActorLocation` (`self.Player`))))
  (if (and (`self.isCollide?`) (not (`self.recharg`)) (not (`self.explode`)))
    (`self.Jump`)
    (if (> _returnvalue_z_2 0.0)
      (if (> _returnvalue_x _returnvalue_x_3)
        (set `self.bisMovingRight` true)
        (else
          (set `self.bisMovingRight` false)))
      (if (`self.bisMovingRight`)
        (`self.K2_SetActorLocation` (`KismetMathLibrary.MakeVector` (+ _returnvalue_x 1.2) _returnvalue_y _returnvalue_z) true)
        (else
          (`self.K2_SetActorLocation` (`KismetMathLibrary.MakeVector` (- _returnvalue_x 1.2) _returnvalue_y _returnvalue_z) true)))
      (else
        (set `self.isCollide?` false)))))

(event `noHead`
  ;[1 1 1] Caminar sin Cabeza
  (if (<= (`self.vida`) 1.0)
    (set `self.nh` true)))

(event `ActiveDesactive`
  ;[1 1 1] Active Desactive
  (if (`self.isDead?`)
    (`self.SpawnPieces`)
    (`PrimitiveComponent.SetCollisionEnabled` (`self.explosion`) "NoCollision")
    (`SceneComponent.SetVisibility` (`self.Sprite`) false true)
    (set `self.explode` false)
    (`PrimitiveComponent.SetCollisionEnabled` (`self.CapsuleComponent`) "NoCollision")
    (set `self.isDead?` false)
    (set `self.vida` 2.0)
    (`self.K2_DestroyActor`)
    (elif (`self.explode`)
      (`PrimitiveComponent.SetCollisionEnabled` (`self.explosion`) "NoCollision")
      (`PrimitiveComponent.SetCollisionEnabled` (`self.CapsuleComponent`) "NoCollision")
      (`KismetSystemLibrary.Delay` 0.4)
      (`self.K2_DestroyActor`))))

(event `moveTo`
  (bind _scalevalue (`self.scaleValue`))
  ;[1 1 1] Movimiento
  (if (`self.Start`)
    (if (`self.Spawn`)
      _
      (elif (`self.isDead?`)
        _
        (elif (`self.isCollide?`)
          _
          (elif (`self.explode`)
            _
            (elif (`self.recharg`)
              _
              (elif (`self.isHit?`)
                _
                (elif (> (.x (`self.K2_GetActorLocation` (`self.Player`))) (.x (`self.K2_GetActorLocation`)))
                  (set `self.bisMovingRight` true)
                  (set `self.scaleValue` 1.0)
                  (`self.AddMovementInput` (1.0 0.0 0.0) _scalevalue)
                  (else
                    (set `self.bisMovingRight` false)
                    (set `self.scaleValue` -1.0)
                    (`self.AddMovementInput` (1.0 0.0 0.0) _scalevalue)))))))))))

(event `UpdateAnimation`
  ;[1 1 1] Update Anim
  (bind _outflipbook (`self.AnimStateMachine` (`self.isHit?`) (`self.nh`) (`self.recharg`) (`self.explode`)))
  (`PaperFlipbookComponent.SetFlipbook` (`self.Sprite`) _outflipbook))

(event `SpawnPieces`
  ;[1 1 1] SpawnPieces
  (`|SpawnActorFromClass` "/Game/AlteredBeast/Blueprints/enemigos/miselanious/leg.leg_C" (`SceneComponent.K2_GetComponentToWorld` (`self.leg`)) "Undefined" "OverrideRootScale" null null)
  (`|SpawnActorFromClass` "/Game/AlteredBeast/Blueprints/enemigos/miselanious/torso.torso_C" (`SceneComponent.K2_GetComponentToWorld` (`self.torso`)) "Undefined" "OverrideRootScale" null null)
  (`|SpawnActorFromClass` "/Game/AlteredBeast/Blueprints/enemigos/miselanious/arm.arm_C" (`SceneComponent.K2_GetComponentToWorld` (`self.arm`)) "Undefined" "OverrideRootScale" null null))

(event `self.ReceiveAnyDamage`
  (params (Damage :type "Float (single-precision)") (DamageType :type "DamageType Object Reference") (InstigatedBy :type "Controller Object Reference") (DamageCauser :type "Actor Object Reference"))
  ;[1 1 1] Recibir Daño
  (if (`self.Start`)
    (if (not (`self.Spawn`))
      (cast `/Game/AlteredBeast/Blueprints/Player1` DamageCauser
        (:`then`
          _)
        (:`CastFailed`
          (cast `/Game/AlteredBeast/Blueprints/Players/proyectile/LoboProyectil` DamageCauser)))
      (set `self.isHit?` true)
      (set `self.vida` (- (`self.vida`) Damage))
      (`GameplayStatics.PlaySoundAtLocation` (`self.sfx_golpe`)))))

(event `Explotar`
  (bind _explosion (`self.explosion`))
  (bind _explosion_2 (`self.explosion`))
  ;[1 1 1] Dañar
  (if (`self.Spawn`)
    _
    (elif (`self.isDead?`)
      _
      (elif (`self.explode`)
        (`PrimitiveComponent.SetCollisionEnabled` _explosion "QueryAndPhysics")
        (`SceneComponent.SetWorldScale3D` _explosion (2.0 3.0 3.0))
        (`PrimitiveComponent.SetCollisionEnabled` (`self.CapsuleComponent`) "NoCollision")
        (for _array_element (`PrimitiveComponent.GetOverlappingActors` _explosion_2 "/Game/AlteredBeast/Blueprints/Player1.Player1_C")
          (if (`PrimitiveComponent.IsOverlappingActor` _explosion_2 _array_element)
            (`GameplayStatics.ApplyDamage` _array_element 1.0 (`self.GetController`) self)))))))

(event `distance`
  (bind _player (`self.Player`))
  ;[1 1 1] Recharg
  (if (`self.Start`)
    (if (`self.Spawn`)
      _
      (elif (`self.isCollide?`)
        _
        (elif (`self.explode`)
          _
          (elif (`self.recharg`)
            _
            (elif (<= (`self.GetHorizontalDistanceTo` _player self) 35.0)
              (if (< (`self.GetVerticalDistanceTo` _player self) 12.0)
                (set `self.recharg` true)))))))))

(event `SpawnEnemy`
  (bind _z (.z (`self.K2_GetActorLocation`)))
  ;[1 1 1] Spawn
  (if (`self.Spawn`)
    (if (<= _z -43.0)
      (`self.K2_SetActorLocation` (`KismetMathLibrary.MakeVector` (.x (`self.K2_GetActorLocation`)) (.y (`self.K2_GetActorLocation`)) (+ _z 3.0)))
      (`PrimitiveComponent.SetCollisionEnabled` (`self.CapsuleComponent`) "QueryAndPhysics"))))

(event `ActivarZombi`
  ;[1 1 1] ACtivar Zombie
  (if (`self.Spawn`)
    (if (>= (.z (`self.K2_GetActorLocation`)) -43.0)
      (`self.K2_SetActorLocation` (`KismetMathLibrary.MakeVector` (.x (`self.K2_GetActorLocation`)) (.y (`self.K2_GetActorLocation`)) -40.0))
      (set `self.Spawn` false)
      (`PrimitiveComponent.SetEnableGravity` (`self.CapsuleComponent`) true)
      (set `CharacterMovementComponent.GravityScale` 1.0 (`self.CharacterMovement`)))))

(event `activarSpawn`
  (if (`self.Start`)
    (set `self.Spawn` true)))

(event `startEvent`
  (set `self.Start` true)
  (`self.activarSpawn`))

(event `self.cercania.OnComponentBeginOverlap`
  (params (OverlappedComponent :type "PrimitiveComponent Object Reference") (OtherActor :type "Actor Object Reference") (OtherComp :type "PrimitiveComponent Object Reference") (OtherBodyIndex :type Integer) (bFromSweep :type Boolean) (SweepResult :type "HitResult Structure (by ref)"))
  (bind _asplayer_1 (cast `/Game/AlteredBeast/Blueprints/Player1` OtherActor))
  (set `self.Player` _asplayer_1))

(event `self.CapsuleComponent.OnComponentBeginOverlap`
  (params (OverlappedComponent :type "PrimitiveComponent Object Reference") (OtherActor :type "Actor Object Reference") (OtherComp :type "PrimitiveComponent Object Reference") (OtherBodyIndex :type Integer) (bFromSweep :type Boolean) (SweepResult :type "HitResult Structure (by ref)"))
  (cast `/Game/AlteredBeast/Blueprints/Player1` OtherActor)
  (if (`KismetStringLibrary.EqualEqual_StrStr` (`KismetSystemLibrary.GetObjectName` OtherComp) "CollisionCylinder")
    (set `self.isCollide?` true)))

(fn `AnimStateMachine`
  (params (`isHIt?` :type Boolean) (`nh?` :type Boolean) (`recharg?` :type Boolean) (explode :type Boolean))
  (returns (OutFLipbook :type "PaperFlipbook Object Reference"))
  (bind _outflipbook (`self.EnumManager`))
  (if explode
    (set `self.EnumMachine` "NewEnumerator6")
    (elif `isHIt?`
      (set `self.EnumMachine` "NewEnumerator3")
      (elif `nh?`
        (if `recharg?`
          (set `self.EnumMachine` "NewEnumerator5")
          (else
            (set `self.EnumMachine` "NewEnumerator2")))
        (elif (`self.recharg`)
          (set `self.EnumMachine` "NewEnumerator4")
          (else
            (set `self.EnumMachine` "NewEnumerator1"))))))
  (return _outflipbook))

(fn `ChosePlayer`
  (if (`self.isChose`)
    (bind _outactors (`GameplayStatics.GetAllActorsOfClass` "/Game/AlteredBeast/Blueprints/Player1.Player1_C"))
    (for _array_element _outactors
      (if (`/Game/AlteredBeast/Blueprints/Player1.yaExiste` _array_element)
        (set `self.Player` _array_element)
        (set `self.isChose` false)
        (break)
        (else
          (set `self.isChose` true))))))

(fn `EnumManager`
  (returns (OutFlipBook :type "PaperFlipbook Object Reference"))
  (return (select `/Game/AlteredBeast/Blueprints/enemigos/Zombie/E_zombie` (`self.EnumMachine`) :`NewEnumerator0` (`self.fb_idle`) :`NewEnumerator1` (`self.fb_walk`) :`NewEnumerator2` (`self.fb_walk_nh`) :`NewEnumerator3` (`self.fb_hit`) :`NewEnumerator4` (`self.fb_charg_h`) :`NewEnumerator5` (`self.fb_charg_nh`) :`NewEnumerator6` (`self.fb_explosion`))))

(fn `ManejoAnimacion`
  (`self.UpdateAnimation`)
  (if (`self.bisMovingRight`)
    (`SceneComponent.K2_SetWorldRotation` (`self.Sprite`) (`KismetMathLibrary.MakeRotator` 0.0 0.0 180.0) false false)
    (else
      (`SceneComponent.K2_SetWorldRotation` (`self.Sprite`) (`KismetMathLibrary.MakeRotator` 0.0) false false)))
  (return))

(fn `UserConstructionScript`
  (`parent.UserConstructionScript`))