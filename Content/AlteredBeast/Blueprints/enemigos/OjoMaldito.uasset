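; OjoMaldito is a flipbook-animated flying eye enemy for an Altered Beast-style game that drifts along X and Z in move, slow and stop phases.
; Tick drives movement, death and animation, mapping state flags to an enum-selected flipbook.
; Delays based on flipbook length clear flags and destroy the dead eye.
; Player or wolf-projectile hits reduce Vida, while overlapping the player deals damage and then kills the eye.
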(event `stopAnim`
  (bind _returnvalue (`self.EnumManager`))
  (if (`self.isDead?`)
    (bind _returnvalue_2 (`PaperFlipbook.GetTotalDuration` _returnvalue))
    (`KismetSystemLibrary.Delay` _returnvalue_2)
    (`self.K2_DestroyActor`)
    (elif (`self.hit?`)
      (`KismetSystemLibrary.Delay` _returnvalue_2)
      (set `self.hit?` false)
      (elif (`self.slow?`)
        (`KismetSystemLibrary.Delay` _returnvalue_2)
        (set `self.slow?` false)
        (elif (not (`self.move?`))
          (`KismetSystemLibrary.Delay` _returnvalue_2)
          (set `self.move?` true))))))

(event `self.ReceiveTick`
  (params (DeltaSeconds :type "Float (single-precision)"))
  (`parent.ReceiveTick` DeltaSeconds)
  (`self.death`)
  (`self.ManejoAnim`)
  (`self.stopAnim`)
  (`self.MoveEye`)
  (`self.DañarPlayer`))

(event `UpdateAnimation`
  (bind _returnvalue (`self.AnimStateMachine`))
  (`PaperFlipbookComponent.SetFlipbook` (`self.Sprite`) _returnvalue))

(event `death`
  (if (<= (`self.vida`) 0.0)
    (`PrimitiveComponent.SetCollisionEnabled` (`self.daño`) "NoCollision")
    (set `self.isDead?` true)))

(event `MoveEye`
  (bind (_returnvalue_x _returnvalue_y _returnvalue_z) (`KismetMathLibrary.BreakVector` (`self.K2_GetActorLocation`)))
  (if (`self.move?`)
    (if (not (`self.hit?`))
      (`self.K2_SetActorLocation` (`KismetMathLibrary.MakeVector` (- _returnvalue_x 1.8) _returnvalue_y (- _returnvalue_z (`self.speed`))) true)
      (`KismetSystemLibrary.Delay` 0.8)
      (set `self.slow?` true)
      (set `self.move?` false))))

(event `self.ReceiveAnyDamage`
  (params (Damage :type "Float (single-precision)") (DamageType :type "DamageType Object Reference") (InstigatedBy :type "Controller Object Reference") (DamageCauser :type "Actor Object Reference"))
  (cast `/Game/AlteredBeast/Blueprints/Player1` DamageCauser
    (:`then`
      (set `self.hit?` true))
    (:`CastFailed`
      (cast `/Game/AlteredBeast/Blueprints/Players/proyectile/LoboProyectil` DamageCauser)
      (set `self.hit?` true)))
  (set `self.vida` (- (`self.vida`) 1.0)))

(event `DañarPlayer`
  (bind `_daño` (`self.daño`))
  (if (not (`self.isDead?`))
    (for _array_element (`PrimitiveComponent.GetOverlappingActors` `_daño` "/Game/AlteredBeast/Blueprints/Player1.Player1_C")
      (bind _asplayer_1 (cast `/Game/AlteredBeast/Blueprints/Player1` _array_element))
      (if (`PrimitiveComponent.IsOverlappingComponent` `_daño` (`Character.CapsuleComponent` _asplayer_1))
        (`GameplayStatics.ApplyDamage` _array_element 2.0 (`self.GetController`) self)
        (`KismetSystemLibrary.Delay` 0.2)
        (set `self.vida` 0.0)))))

(fn `AnimStateMachine`
  (returns (ReturnValue :type "PaperFlipbook Object Reference"))
  (bind _returnvalue (`self.EnumManager`))
  (if (`self.isDead?`)
    (set `self.EnumMachine` "NewEnumerator3")
    (elif (`self.move?`)
      (if (`self.hit?`)
        (set `self.EnumMachine` "NewEnumerator5")
        (else
          (set `self.EnumMachine` "NewEnumerator0")))
      (elif (`self.slow?`)
        (if (`self.hit?`)
          (set `self.EnumMachine` "NewEnumerator7")
          (else
            (set `self.EnumMachine` "NewEnumerator4")))
        (elif (`self.hit?`)
          (set `self.EnumMachine` "NewEnumerator6")
          (else
            (set `self.EnumMachine` "NewEnumerator1"))))))
  (return _returnvalue))

(fn `EnumManager`
  (returns (ReturnValue :type "PaperFlipbook Object Reference"))
  (return (select `/Game/AlteredBeast/Blueprints/enemigos/E_ojomaldito` (`self.EnumMachine`) :`NewEnumerator0` (`self.fb_move`) :`NewEnumerator1` (`self.fb_stop`) :`NewEnumerator4` (`self.fb_slow`) :`NewEnumerator3` (`self.fb_death`) :`NewEnumerator5` (`self.fb_hit_move`) :`NewEnumerator6` (`self.fb_hit_stop`) :`NewEnumerator7` (`self.fb_hit_slow`))))

(fn `ManejoAnim`
  (`self.UpdateAnimation`))

(fn `UserConstructionScript`
  (`parent.UserConstructionScript`))