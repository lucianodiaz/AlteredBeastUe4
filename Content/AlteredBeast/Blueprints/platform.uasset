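; Platform for an Altered Beast game that is passable to pawns until a qualifying character enters its trigger box.
; The Plata component ignores the Pawn channel at start, blocks it when Player1 or an enemigo not named "agar" enters Box, and ignores it again when either class exits.
; The response is one shared toggle with no occupant count, so any such exit opens the platform for every pawn.
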(event `self.ReceiveBeginPlay`
  (`PrimitiveComponent.SetCollisionResponseToChannel` (`self.plata`) "ECC_Pawn" "ECR_Ignore"))

(event `self.Box.OnComponentBeginOverlap`
  (params (OverlappedComponent :type "PrimitiveComponent Object Reference") (OtherActor :type "Actor Object Reference") (OtherComp :type "PrimitiveComponent Object Reference") (OtherBodyIndex :type Integer) (bFromSweep :type Boolean) (SweepResult :type "HitResult Structure (by ref)"))
  (cast `/Game/AlteredBeast/Blueprints/Player1` OtherActor
    (:`then`
      (`PrimitiveComponent.SetCollisionResponseToChannel` (`self.plata`) "ECC_Pawn" "ECR_Block"))
    (:`CastFailed`
      (bind _asenemigo (cast `/Game/AlteredBeast/Blueprints/enemigos/enemigo` OtherActor))
      (if (`KismetStringLibrary.NotEqual_StrStr` (`KismetSystemLibrary.GetDisplayName` _asenemigo) "agar")
        (`PrimitiveComponent.SetCollisionResponseToChannel` (`self.plata`) "ECC_Pawn" "ECR_Block")))))

(event `self.Box.OnComponentEndOverlap`
  (params (OverlappedComponent :type "PrimitiveComponent Object Reference") (OtherActor :type "Actor Object Reference") (OtherComp :type "PrimitiveComponent Object Reference") (OtherBodyIndex :type Integer))
  (cast `/Game/AlteredBeast/Blueprints/Player1` OtherActor
    (:`then`
      (`PrimitiveComponent.SetCollisionResponseToChannel` (`self.plata`) "ECC_Pawn" "ECR_Ignore"))
    (:`CastFailed`
      (cast `/Game/AlteredBeast/Blueprints/enemigos/enemigo` OtherActor)
      (`PrimitiveComponent.SetCollisionResponseToChannel` (`self.plata`) "ECC_Pawn" "ECR_Ignore"))))

(fn `UserConstructionScript`)