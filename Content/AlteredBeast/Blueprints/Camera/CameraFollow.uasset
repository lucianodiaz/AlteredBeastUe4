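; Auto-scrolling follow camera actor for Altered Beast that advances along X while its move flag is set.
; Each tick it picks a speed tier from the player's distance to the rear box, moving faster as that gap grows.
; The rear box pushes a living player on hit, and either box can reassign the tracked Player1 found after BeginPlay.
; CameraSelect makes this actor the view target.
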(event `velocityCamera`
  (bind _returnvalue (`KismetMathLibrary.Abs` (- (.x (`SceneComponent.K2_GetComponentLocation` (`self.caja atras`))) (.x (`SceneComponent.K2_GetComponentLocation` (`Character.CapsuleComponent` (`self.player`)))))))
  (if (!= (`self.player`) null)
    (if (`self.MOve`)
      (if (<= _returnvalue 90.0)
        (set `self.velocity` 0.03)
        (elif (and (> _returnvalue 90.0) (<= _returnvalue 150.0))
          (set `self.velocity` 0.04)
          (elif (and (> _returnvalue 180.0) (<= _returnvalue 300.0))
            (set `self.velocity` 0.25)
            (elif (> _returnvalue 300.0)
              (set `self.velocity` 0.35))))))))

(event `self.ReceiveBeginPlay`
  (`KismetSystemLibrary.Delay` 1.0)
  (bind _outactors (`GameplayStatics.GetAllActorsOfClass` "/Game/AlteredBeast/Blueprints/Player1.Player1_C"))
  (for _array_element _outactors
    (if (`/Game/AlteredBeast/Blueprints/Player1.yaExiste` _array_element)
      (set `self.player` _array_element))))

(event `self.ReceiveTick`
  (params (DeltaSeconds :type "Float (single-precision)"))
  (if (`self.MOve`)
    (`self.velocityCamera`)
    (`self.moveCamera` DeltaSeconds)))

(event `moveCamera`
  (params (dt :type "Float (double-precision)"))
  (`self.K2_SetActorLocation` self (`KismetMathLibrary.MakeVector` (+ (.x (`self.K2_GetActorLocation` self)) dt (`self.velocity`))) false false))

(event `self.caja adelante.OnComponentHit`
  (params (HitComponent :type "PrimitiveComponent Object Reference") (OtherActor :type "Actor Object Reference") (OtherComp :type "PrimitiveComponent Object Reference") (NormalImpulse :type "Vector Structure") (Hit :type "HitResult Structure (by ref)"))
  (bind _asplayer_1 (cast `/Game/AlteredBeast/Blueprints/Player1` OtherActor))
  (set `self.player` _asplayer_1))

(event `self.caja atras.OnComponentHit`
  (params (HitComponent :type "PrimitiveComponent Object Reference") (OtherActor :type "Actor Object Reference") (OtherComp :type "PrimitiveComponent Object Reference") (NormalImpulse :type "Vector Structure") (Hit :type "HitResult Structure (by ref)"))
  (bind _asplayer_1 (cast `/Game/AlteredBeast/Blueprints/Player1` OtherActor))
  (if (not (`/Game/AlteredBeast/Blueprints/Player1.IsDeath` _asplayer_1))
    (bind _output_get (set `self.player` _asplayer_1))
    (`PrimitiveComponent.SetAllPhysicsLinearVelocity` (`Character.CapsuleComponent` _output_get) NormalImpulse true)
    (set `/Game/AlteredBeast/Blueprints/Player1.bisMoving?` true _asplayer_1)))

(fn `CameraSelect`
  (params (Player :type Integer))
  (`PlayerController.SetViewTargetWithBlend` (`GameplayStatics.GetPlayerController` Player) self 0.0 "VTBlend_Linear" 0.0 false))

(fn `UserConstructionScript`)