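; Destructible rock obstacle that rises to a fixed height when StartEvent is triggered and breaks apart when its life runs out.
; Tick drives the rise, a random X-axis shake while hit, a delayed reset to the stored X, and the death check.
; Box overlaps subtract life for player punches and kicks, skull punches, wolf projectiles and birds.
; On death it spawns five smaller rock pieces at marker components, then destroys itself.
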(event `self.ReceiveBeginPlay`
  (`self.stayInTheMiddle`)
  (set `self.PosX` (.x (`SceneComponent.K2_GetComponentLocation` (`self.RenderComponent`)))))

(event `self.ReceiveTick`
  (params (DeltaSeconds :type "Float (single-precision)"))
  (`self.Spawn`)
  (`self.ActivarRoca`)
  (`self.Hit`)
  (`self.StopFight`)
  (`self.isDeath`))

(event `StopFight`
  (if (`self.Golpe`)
    (`KismetSystemLibrary.Delay` 0.5)
    (set `self.Golpe` false)
    (`self.K2_SetActorLocation` (`KismetMathLibrary.MakeVector` (`self.PosX`) (.y (`SceneComponent.K2_GetComponentLocation` (`self.RenderComponent`))) (.z (`SceneComponent.K2_GetComponentLocation` (`self.RenderComponent`)))))))

(event `Spawn`
  (bind _z (.z (`self.K2_GetActorLocation`)))
  ;[1 1 1] Aparecer
  (if (`self.bSpawn`)
    (if (<= _z -49.0)
      (`self.K2_SetActorLocation` (`KismetMathLibrary.MakeVector` (.x (`self.K2_GetActorLocation`)) (.y (`self.K2_GetActorLocation`)) (+ _z 3.0))))))

(event `activarSpawn`
  (if (`self.Start`)
    (set `self.bSpawn` true)))

(event `StartEvent`
  (set `self.Start` true)
  (`self.activarSpawn`))

(event `ActivarRoca`
  ;[1 1 1] Frenar
  (if (`self.bSpawn`)
    (if (>= (.z (`self.K2_GetActorLocation`)) -47.0)
      (`self.K2_SetActorLocation` (`KismetMathLibrary.MakeVector` (.x (`self.K2_GetActorLocation`)) (.y (`self.K2_GetActorLocation`)) -49.0))
      (set `self.bSpawn` false))))

(event `Hit`
  (if (`self.Golpe`)
    (`self.K2_SetActorLocation` (`KismetMathLibrary.MakeVector` (+ (.x (`SceneComponent.K2_GetComponentLocation` (`self.RenderComponent`))) (`KismetMathLibrary.RandomFloatInRange` -0.5 0.5)) (.y (`SceneComponent.K2_GetComponentLocation` (`self.RenderComponent`))) (.z (`SceneComponent.K2_GetComponentLocation` (`self.RenderComponent`)))))))

(event `self.caja.OnComponentBeginOverlap`
  (params (OverlappedComponent :type "PrimitiveComponent Object Reference") (OtherActor :type "Actor Object Reference") (OtherComp :type "PrimitiveComponent Object Reference") (OtherBodyIndex :type Integer) (bFromSweep :type Boolean) (SweepResult :type "HitResult Structure (by ref)"))
  (bind _returnvalue (`KismetSystemLibrary.GetObjectName` OtherComp))
  (bind _sfx_golpe (`self.sfx_golpe`))
  ;[1 1 1] Verificar golpe
  (bind _asplayer_1 (cast `/Game/AlteredBeast/Blueprints/Player1` OtherActor)
    (:`then`
      (if (`self.Golpe`)
        _
        (elif (`KismetStringLibrary.EqualEqual_StrStr` _returnvalue "punch")
          (bind _hit (`/Game/AlteredBeast/Blueprints/Player1.hit` _asplayer_1))
          (set `self.life` (- (`self.life`) _hit))
          (`GameplayStatics.PlaySoundAtLocation` _sfx_golpe)
          (set `self.Golpe` true)
          (elif (`KismetStringLibrary.EqualEqual_StrStr` _returnvalue "kick")
            (set `self.life` (- (`self.life`) _hit) :!label _label)
            (`GameplayStatics.PlaySoundAtLocation` _sfx_golpe)
            (set `self.Golpe` true)
            (elif (`KismetStringLibrary.EqualEqual_StrStr` (`KismetSystemLibrary.GetObjectName` OtherComp) "megaKick")
              (goto _label))))))
    (:`CastFailed`
      (cast `/Game/AlteredBeast/Blueprints/enemigos/skull/skull` OtherActor
        (:`then`
          (if (`KismetStringLibrary.EqualEqual_StrStr` (`KismetSystemLibrary.GetObjectName` OtherComp) "punch")
            (set `self.life` (- (`self.life`) 1.0))
            (set `self.Golpe` true)))
        (:`CastFailed`
          (cast `/Game/AlteredBeast/Blueprints/Players/proyectile/LoboProyectil` OtherActor
            (:`then`
              (set `self.life` (- (`self.life`) 3.0))
              (set `self.Golpe` true))
            (:`CastFailed`
              (cast `/Game/AlteredBeast/Blueprints/enemigos/pajaro/pajaro` OtherActor)
              (set `self.life` (- (`self.life`) 1.0))
              (set `self.Golpe` true))))))))

(fn `isDeath`
  (if (`self.bSpawn`)
    _
    (elif (<= (`self.life`) 0.0)
      (`self.spawnRock` (`KismetMathLibrary.MakeTransform` (.location (`SceneComponent.K2_GetComponentToWorld` (`self.rock1`))) (.rotation (`SceneComponent.K2_GetComponentToWorld` (`self.rock1`))) (0.3 0.3 0.3)))
      (`self.spawnRock` (`KismetMathLibrary.MakeTransform` (.location (`SceneComponent.K2_GetComponentToWorld` (`self.rock2`))) (.rotation (`SceneComponent.K2_GetComponentToWorld` (`self.rock2`))) (0.3 0.3 0.3)) 1.0)
      (`self.spawnRock` (`KismetMathLibrary.MakeTransform` (.location (`SceneComponent.K2_GetComponentToWorld` (`self.rock3`))) (.rotation (`SceneComponent.K2_GetComponentToWorld` (`self.rock3`))) (0.3 0.3 0.3)) 2.0)
      (`self.spawnRock` (`KismetMathLibrary.MakeTransform` (.location (`SceneComponent.K2_GetComponentToWorld` (`self.rock4`))) (struct) (0.3 0.3 0.3)) 3.0)
      (`self.spawnRock` (`KismetMathLibrary.MakeTransform` (.location (`SceneComponent.K2_GetComponentToWorld` (`self.rock5`))) (.rotation (`SceneComponent.K2_GetComponentToWorld` (`self.rock5`))) (0.3 0.3 0.3)) 4.0)
      (`self.K2_DestroyActor`))))

(fn `spawnRock`
  (params (RockTransform :type "Transform Structure") (number :type "Float (double-precision)"))
  (`|MultiGate` false false (`KismetMathLibrary.FTrunc` number)
    (:`Out 0`
      (`|SpawnActorFromClass` (`|GetArrayItem` (`self.rock`)) RockTransform "Undefined" "OverrideRootScale" null null))
    (:`Out 1`
      (`|SpawnActorFromClass` (`|GetArrayItem` (`self.rock`) 1) RockTransform "Undefined" "OverrideRootScale" null null))
    (:`Out 2`
      (`|SpawnActorFromClass` (`|GetArrayItem` (`self.rock`) 2) RockTransform "Undefined" "OverrideRootScale" null null))
    (:`Out 3`
      (`|SpawnActorFromClass` (`|GetArrayItem` (`self.rock`) 3) RockTransform "Undefined" "OverrideRootScale" null null))
    (:`Out 4`
      (`|SpawnActorFromClass` (`|GetArrayItem` (`self.rock`)) RockTransform "Undefined" "OverrideRootScale" null null))))

(fn `stayInTheMiddle`
  (bind (_returnvalue_x _returnvalue_y _returnvalue_z) (`KismetMathLibrary.BreakVector` (`self.K2_GetActorLocation`)))
  (`self.K2_SetActorLocation` (`KismetMathLibrary.MakeVector` _returnvalue_x 40.0 _returnvalue_z)))

(fn `UserConstructionScript`)