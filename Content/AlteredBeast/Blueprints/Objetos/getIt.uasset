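; Floating pickup actor that plays the power-up collected sound and destroys itself when Player1 overlaps its sphere, applying no effect to the player here.
; Each Tick pins Y to a fixed plane and raises the actor with a swept move, while a wrapping Clock counter swings it along X.
; Motion is per-frame, without delta-time scaling.
; A Delay in Tick destroys it after 30 seconds if uncollected.
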(event `clocks`
  (if (> (`self.clock`) 3.0)
    (set `self.clock` -3.0)))

(event `self.ReceiveTick`
  (params (DeltaSeconds :type "Float (single-precision)"))
  (`self.stayInTheMiddle`)
  (set `self.clock` (+ (`self.clock`) 0.1))
  (`self.clocks`)
  (`self.K2_SetActorLocation` (`KismetMathLibrary.MakeVector` (- (.x (`self.K2_GetActorLocation`)) (`self.clock`)) (.y (`self.K2_GetActorLocation`)) (+ (.z (`self.K2_GetActorLocation`)) 0.6)) true)
  (`KismetSystemLibrary.Delay` 30.0)
  (`self.K2_DestroyActor`))

(event `self.Sphere.OnComponentBeginOverlap`
  (params (OverlappedComponent :type "PrimitiveComponent Object Reference") (OtherActor :type "Actor Object Reference") (OtherComp :type "PrimitiveComponent Object Reference") (OtherBodyIndex :type Integer) (bFromSweep :type Boolean) (SweepResult :type "HitResult Structure (by ref)"))
  (cast `/Game/AlteredBeast/Blueprints/Player1` OtherActor)
  (`GameplayStatics.PlaySoundAtLocation` "/Game/AlteredBeast/sfx/power_up_recolectado_Cue.power_up_recolectado_Cue")
  (`self.K2_DestroyActor`))

(fn `stayInTheMiddle`
  (`self.K2_SetActorLocation` (`KismetMathLibrary.MakeVector` (.x (`self.K2_GetActorLocation`)) 40.0 (.z (`self.K2_GetActorLocation`)))))

(fn `UserConstructionScript`)