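; Level manager for an Altered Beast game that runs player joining, transformations, game over and level progression.
; BeginPlay gathers players and game-instance counts, then Tick polls every system, moving up to four players to start points.
; Transformations play level-specific wolf or dragon videos while enemies freeze.
; Boss Agar's state swaps backgrounds and opens the next level; excess deaths trigger slow motion and return to the menu.
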(event `OpenVideo`
  (params (MP :type "MediaPlayer Object Reference") (MS :type "FileMediaSource Object Reference"))
  ;[1 1 1] StopVideo
  (`MediaPlayer.OpenSource` MP MS))

(event `FrenarVideo`
  ;[1 1 1] StopVideo
  (if (`self.ReproduceVideo`)
    (switch `int` (`self.nivel`)
      (:`Default`
        (`self.OpenVideo` (`self.MP_Lobo`) (`self.MS_Lobo`) :!label _label)
        (bind _foundwidgets (`WidgetBlueprintLibrary.GetAllWidgetsOfClass` "/Game/AlteredBeast/GUI/TransformacionLoboUI.TransformacionLoboUI_C" false))
        (`KismetArrayLibrary.Array_RemoveItem` _foundwidgets (`|GetArrayItem` _foundwidgets)))
      (:`1`
        (goto _label))
      (:`2`
        (`self.OpenVideo` (`self.MP_dragon`) (`self.MS_dragon`))
        (bind _foundwidgets_2 (`WidgetBlueprintLibrary.GetAllWidgetsOfClass` "/Game/AlteredBeast/GUI/TransformacionDragonUI.TransformacionDragonUI_C" false))
        (`KismetArrayLibrary.Array_RemoveItem` _foundwidgets_2 (`|GetArrayItem` _foundwidgets_2))))
    (set `self.ReproduceVideo` false)
    (`KismetSystemLibrary.Delay` 1.4)
    (bind _outactors (`GameplayStatics.GetAllActorsOfClass` "/Game/AlteredBeast/Blueprints/enemigos/enemigo.enemigo_C"))
    (for _array_element _outactors
      (set `/Game/AlteredBeast/Blueprints/enemigos/enemigo.Stop` false _array_element))))

(event `self.ReceiveBeginPlay`
  ;[1 1 1] BeginPlay
  (bind _ascant_player_2 (cast `/Game/AlteredBeast/GameInstance/cantPlayer2` (`GameplayStatics.GetGameInstance`)))
  (set `self.CantPlayers` (`/Game/AlteredBeast/GameInstance/cantPlayer2.cantPlayer` _ascant_player_2))
  (set `self.MasPlayers` (`/Game/AlteredBeast/GameInstance/cantPlayer2.maxPlayer` _ascant_player_2))
  (set `self.MS_dragon` "/Game/Movies/TransformacionDragon.TransformacionDragon")
  (set `self.MP_dragon` "/Game/Movies/MP_DragonTransformacion.MP_DragonTransformacion")
  (set `self.MS_Lobo` "/Game/Movies/transformacionLobo.transformacionLobo")
  (set `self.MP_Lobo` "/Game/Movies/MP_LoboTransformacion.MP_LoboTransformacion")
  (bind _returnvalue (`|CreateWidget` "/Game/AlteredBeast/GUI/LifePoints.LifePoints_C" (`GameplayStatics.GetPlayerController` 0)))
  (`UserWidget.AddToPlayerScreen` _returnvalue 0)
  (`SceneComponent.SetVisibility` (`PaperSpriteActor.RenderComponent` (`self.Spritefront_0`)) false false)
  (`SceneComponent.SetVisibility` (`PaperSpriteActor.RenderComponent` (`self.Spritefront_0`)) false false)
  (bind _asalteredbeastgm (cast `/Game/AlteredBeast/gamemode/alteredbeastgm` (`GameplayStatics.GetGameMode`)))
  (`/Game/AlteredBeast/gamemode/alteredbeastgm.spawn Players` _asalteredbeastgm)
  (bind _outactors (`GameplayStatics.GetAllActorsOfClass` "/Game/AlteredBeast/Blueprints/Player1.Player1_C"))
  (for _array_element _outactors
    (`KismetArrayLibrary.Array_Add` (`self.Players`) _array_element)))

(event `MenuGOver`
  ;[1 1 1] perdiste? volve al menu principal
  (if (`self.MenuOver`)
    (`PlayerCameraManager.StartCameraFade` :`self` (`PlayerController.PlayerCameraManager` (`GameplayStatics.GetPlayerController` 0)) :`ToAlpha` 1.0 :`Duration` 0.5)
    (`GameplayStatics.OpenLevel` "Menu" false)))

(event `self.ReceiveTick`
  (params (DeltaSeconds :type "Float (single-precision)"))
  ;[1 1 1] EveryTick
  (`self.MenuGOver`)
  (`self.SpawnPlayers`)
  (`self.GameOVER`)
  (`self.Blackback`)
  (`self.WhiteBack`)
  (`self.reproducirTransformacion`)
  (`self.FrenarVideo`)
  (`self.PasarAotroNivel`))

(event `reproducirTransformacion`
  (bind _musicmanager (`self.MusicManager`))
  ;[1 1 1] Reproducir transformacion
  (for _array_element (`self.Players`)
    (if (`/Game/AlteredBeast/Blueprints/Player1.yaExiste` _array_element)
      (if (and (`/Game/AlteredBeast/Blueprints/Player1.bTransformacion` _array_element) (not (`/Game/AlteredBeast/Blueprints/Player1.bishuman?` _array_element)))
        (set `self.ReproduceVideo` true)
        (switch `int` (`self.nivel`)
          (:`Default`
            (bind _returnvalue (`|CreateWidget` "/Game/AlteredBeast/GUI/TransformacionLoboUI.TransformacionLoboUI_C" (`GameplayStatics.GetPlayerController` (`/Game/AlteredBeast/Blueprints/Player1.playerInt` _array_element)) _musicmanager (`self.MP_Lobo`) :!label _label_2))
            (`UserWidget.AddToPlayerScreen` _returnvalue 0))
          (:`1`
            (goto _label_2))
          (:`2`
            (bind _returnvalue_2 (`|CreateWidget` "/Game/AlteredBeast/GUI/TransformacionDragonUI.TransformacionDragonUI_C" null (`self.MP_dragon`) _musicmanager))
            (`UserWidget.AddToPlayerScreen` _returnvalue_2 0)))
        (bind _outactors (`GameplayStatics.GetAllActorsOfClass` "/Game/AlteredBeast/Blueprints/enemigos/enemigo.enemigo_C"))
        (for _array_element_2 _outactors
          (set `/Game/AlteredBeast/Blueprints/enemigos/enemigo.Stop` true _array_element_2))))))

(event `GetDeaths`
  (params (muerto :type Integer))
  (bind _returnvalue (+ muerto (`self.muertos`)))
  ;[1 1 1] Obtener Muertos
  (if (> _returnvalue 0)
    (set `self.muertos` _returnvalue)))

(event `obtenerCantMonster`
  (params (monstruo :type Integer))
  ;[1 1 1] Obtener cantidad de monstruos
  (set `self.Monstruos` (+ monstruo (`self.Monstruos`))))

(event `PasarAotroNivel`
  (bind _agar (`self.agar`))
  (bind _nivel (`self.nivel`))
  ;[1 1 1] NextLevel
  (if (`/Game/AlteredBeast/Blueprints/enemigos/enemigo.isDead?` _agar)
    (bind _outactors (`GameplayStatics.GetAllActorsOfClass` "/Game/AlteredBeast/Blueprints/Player1.Player1_C"))
    (for _array_element _outactors
      (set `/Game/AlteredBeast/Blueprints/Player1.IA` true _array_element))
    (if (`/Game/AlteredBeast/Blueprints/enemigos/Agar/agar.End` _agar)
      (if (< (`self.nivel`) (`self.maxNiveles`))
        (`GameplayStatics.OpenLevel` (`KismetSystemLibrary.MakeLiteralName` (`KismetStringLibrary.Conv_StringToName` (`KismetStringLibrary.Concat_StrStr` "leveltrans" (`KismetStringLibrary.Conv_IntToString` _nivel) (`KismetStringLibrary.Conv_IntToString` (+ _nivel 1))))))
        (else
          (`PlayerCameraManager.StartCameraFade` :`self` (`PlayerController.PlayerCameraManager` (`GameplayStatics.GetPlayerController` 0)) :`ToAlpha` 1.0 :`Duration` 0.3 :`bShouldFadeAudio` true)
          (`GameplayStatics.OpenLevel` "Menu"))))))

(event `GameOVER`
  ;[1 1 1] gameOver
  (if (> (`self.muertos`) (`self.CantPlayers`))
    (bind _output_get (set `self.GO` true))
    (`GameplayStatics.SetGlobalTimeDilation` 0.1)
    (set `/Game/AlteredBeast/Blueprints/Camera/CameraFollow.MOve` false (`self.CM`))
    (set `/Game/AlteredBeast/music/MusicManager.GOver` _output_get (`self.MusicManager`))
    (`KismetSystemLibrary.Delay` 1.0)
    (set `self.MenuOver` true)))

(event `GMMute`
  (`/Game/AlteredBeast/music/MusicManager.mute` (`self.MusicManager`)))

(event `PauseWorld`
  (params (pause :type Boolean) (time :type "Float (double-precision)"))
  ;[1 1 1] Pause world
  (bind _outactors (`GameplayStatics.GetAllActorsOfClass` "/Game/AlteredBeast/Blueprints/Player1.Player1_C"))
  (for _array_element _outactors
    (set `/Game/AlteredBeast/Blueprints/Player1.NoMove` pause _array_element))
  (set `/Game/AlteredBeast/Blueprints/Camera/CameraFollow.MOve` (not pause) (`self.CM`))
  (bind _outactors_2 (`GameplayStatics.GetAllActorsOfClass` "/Game/AlteredBeast/Blueprints/enemigos/enemigo.enemigo_C"))
  (for _array_element_2 _outactors_2
    (set `/Game/AlteredBeast/Blueprints/enemigos/enemigo.Stop` pause _array_element_2))
  (`/Game/AlteredBeast/music/MusicManager.Pause` (`self.MusicManager`) pause)
  (set `self.Pause` pause)
  (`GameplayStatics.SetGlobalTimeDilation` time))

(fn `Blackback`
  (if (`/Game/AlteredBeast/Blueprints/enemigos/Agar/agar.transformado` (`self.agar`))
    (`SceneComponent.SetVisibility` (`PaperSpriteActor.RenderComponent` (`self.SpriteFondo`)) false false)
    (`SceneComponent.SetVisibility` (`PaperSpriteActor.RenderComponent` (`self.Spritefront`)) false false)
    (`SceneComponent.SetVisibility` (`PaperSpriteActor.RenderComponent` (`self.Spritefront_0`)) true false)
    (`SceneComponent.SetVisibility` (`PaperSpriteActor.RenderComponent` (`self.SpriteFondo_0`)) true false)))

(fn `CreatePlayerBeforeGame`
  (if (`self.MasPlayers`)
    (bind _ascant_player_2 (cast `/Game/AlteredBeast/GameInstance/cantPlayer2` (`GameplayStatics.GetGameInstance`)))
    (for _index (range (+ (`/Game/AlteredBeast/GameInstance/cantPlayer2.cantPlayer` _ascant_player_2) 1))
      (switch `int` _index
        (:`0`
          (`KismetSystemLibrary.PrintText` "jugador 1")
          (bind _output (`|GetArrayItem` (`self.Players`) _index))
          (bind _output_2 (`|GetArrayItem` (`self.posPlayers`) _index))
          (`self.K2_SetActorLocation` _output (`self.K2_GetActorLocation` _output_2) false false))
        (:`1`
          (`KismetSystemLibrary.PrintText` "jugador 2")
          (`self.K2_SetActorLocation` _output (`self.K2_GetActorLocation` _output_2) false false))
        (:`2`
          (`KismetSystemLibrary.PrintText` "jugador 3")
          (`self.K2_SetActorLocation` _output (`self.K2_GetActorLocation` _output_2) false false))
        (:`3`
          (`KismetSystemLibrary.PrintText` "jugador 4")
          (`self.K2_SetActorLocation` _output (`self.K2_GetActorLocation` _output_2) false false)))
      (set `/Game/AlteredBeast/Blueprints/Player1.Aparecer` true _output)
      (`/Game/AlteredBeast/Blueprints/Camera/CameraFollow.CameraSelect` (`self.CM`) _index)
      (set `/Game/AlteredBeast/Blueprints/Player1.yaExiste` true _output)
      (set `/Game/AlteredBeast/Blueprints/Player1.NoMove` false _output)
      (set `self.MasPlayers` false)
      (set `/Game/AlteredBeast/Blueprints/Player1.Aparecer` false _output))))

(fn `createPlayerInGame`
  (params (seleccion :type Integer) (player :type "/Game/AlteredBeast/Blueprints/Player1 Object Reference"))
  (bind _returnvalue (== (`/Game/AlteredBeast/Blueprints/Player1.playerInt` player) (`self.JugadorAaparecer`)))
  (bind _output (`|GetArrayItem` (`self.posPlayers`) seleccion))
  (switch `int` seleccion
    (:`0`
      (if _returnvalue
        (`self.K2_SetActorLocation` player (`self.K2_GetActorLocation` _output) false false)
        (`/Game/AlteredBeast/Blueprints/Camera/CameraFollow.CameraSelect` (`self.CM`) seleccion :!label _label)))
    (:`1`
      (if _returnvalue
        (`self.K2_SetActorLocation` player (`self.K2_GetActorLocation` _output) false false)
        (goto _label)))
    (:`2`
      (if _returnvalue
        (`self.K2_SetActorLocation` player (`self.K2_GetActorLocation` _output) false false)
        (goto _label)))
    (:`3`
      (if _returnvalue
        (`self.K2_SetActorLocation` player (`self.K2_GetActorLocation` _output) false false)
        (goto _label)))))

(fn `LocationPlayer`
  (params (player :type "/Game/AlteredBeast/Blueprints/Player1 Object Reference") (seleccion :type Integer))
  (`self.createPlayerInGame` seleccion player)
  (set `/Game/AlteredBeast/Blueprints/Player1.yaExiste` true player)
  (set `/Game/AlteredBeast/Blueprints/Player1.NoMove` false player)
  (set `/Game/AlteredBeast/Blueprints/Player1.invulnerable` true player)
  (bind _ascant_player_2 (cast `/Game/AlteredBeast/GameInstance/cantPlayer2` (`GameplayStatics.GetGameInstance`)))
  (bind _output_get (set `/Game/AlteredBeast/GameInstance/cantPlayer2.cantPlayer` (+ (`/Game/AlteredBeast/GameInstance/cantPlayer2.cantPlayer` _ascant_player_2) 1) _ascant_player_2))
  (set `self.CantPlayers` _output_get))

(fn `SpawnPlayers`
  (if (`self.Start?`)
    (for _array_element (`self.Players`)
      (set `/Game/AlteredBeast/Blueprints/Player1.HowMonsterIs?` (`self.MonsterSelect`) _array_element)
      (if (`/Game/AlteredBeast/Blueprints/Player1.Aparecer` _array_element)
        (bind _yaexiste (`/Game/AlteredBeast/Blueprints/Player1.yaExiste` _array_element))
        (if (not _yaexiste)
          (bind _output_get (set `self.JugadorAaparecer` (`/Game/AlteredBeast/Blueprints/Player1.playerInt` _array_element)))
          (`self.LocationPlayer` _array_element _output_get))
        (elif (not _yaexiste)
          (`self.CreatePlayerBeforeGame`))))
    (else
      (`/Game/AlteredBeast/Blueprints/Camera/CameraFollow.CameraSelect` (`self.CM`) 0))))

(fn `StopEnemies`
  (bind _outactors (`GameplayStatics.GetAllActorsOfClass` "/Game/AlteredBeast/Blueprints/enemigos/enemigo.enemigo_C"))
  (for _array_element _outactors
    (set `/Game/AlteredBeast/Blueprints/enemigos/enemigo.Stop` true _array_element)))

(fn `StopPlayers`
  (bind _outactors (`GameplayStatics.GetAllActorsOfClass` "/Game/AlteredBeast/Blueprints/Player1.Player1_C"))
  (for _array_element _outactors
    (set `/Game/AlteredBeast/Blueprints/Player1.NoMove` true _array_element)))

(fn `UserConstructionScript`)

(fn `WhiteBack`
  (if (`/Game/AlteredBeast/Blueprints/enemigos/enemigo.isDead?` (`self.agar`))
    (`SceneComponent.SetVisibility` (`PaperSpriteActor.RenderComponent` (`self.SpriteFondo`)) true false)
    (`SceneComponent.SetVisibility` (`PaperSpriteActor.RenderComponent` (`self.Spritefront`)) true false)
    (`SceneComponent.SetVisibility` (`PaperSpriteActor.RenderComponent` (`self.Spritefront_0`)) false false)
    (`SceneComponent.SetVisibility` (`PaperSpriteActor.RenderComponent` (`self.SpriteFondo_0`)) false false)))